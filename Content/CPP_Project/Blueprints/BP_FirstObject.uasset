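; BP_FirstObject is an actor Blueprint that adds disco and floating effects on top of C++ rotation logic.
; BeginPlay calls StartRotating after a short delay.
; DiscoMode, declared in C++, applies a dynamic material and starts a looping timer that randomizes its colour and calls AddRotationSpeed.
; Float plays the Raise timeline to lift and enlarge the actor while brightening that material's emissive.
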(event `self.ReceiveBeginPlay`
  ;[1 1 1] C++ Event Call
  (`KismetSystemLibrary.Delay` 4.0)
  (`self.StartRotating`))

(event `self.DiscoMode`
  ;[1 1 1] C++ Declared Event -> Material Creation & Timer Setup
  (bind _returnvalue (`KismetMaterialLibrary.CreateDynamicMaterialInstance` "/Game/CPP_Project/Materials/M_ColourInst.M_ColourInst"))
  (bind _output_get (set `self.Material` _returnvalue))
  (`PrimitiveComponent.SetMaterial` (`self._Mesh`) 0 _output_get)
  (bind _returnvalue_2 (`KismetSystemLibrary.K2_SetTimerDelegate` (delegate `ChangeColour`) 0.2 true))
  (set `self.Timer` _returnvalue_2))

(event `ChangeColour`
  ;[1 1 1] Dynamic Material
  (`MaterialInstanceDynamic.SetVectorParameterValue` (`self.Material`) "Colour" (make `LinearColor` (`KismetMathLibrary.RandomFloatInRange` 0.0 1.0) (`KismetMathLibrary.RandomFloatInRange` 0.0 1.0) (`KismetMathLibrary.RandomFloatInRange` 0.0 1.0) 1.0))
  (`self.AddRotationSpeed`))

(event `self.Float`
  (bind _startlocation (`self.StartLocation`))
  ;[1 1 1] Floating
  (set `self.StartLocation` (`self.K2_GetActorLocation`))
  (bind (_direction _alpha) (`Timeline|Raise`)
    (:`Update`
      (`self.K2_SetActorLocation` (`KismetMathLibrary.VLerp` _startlocation (+ _startlocation (0.0 0.0 500.0)) _alpha))
      (`MaterialInstanceDynamic.SetScalarParameterValue` (`self.Material`) "Emissive" (`KismetMathLibrary.Lerp` 2.0 30.0 _alpha))
      (`self.SetActorScale3D` (`KismetMathLibrary.VLerp` (1.0 1.0 1.0) (2.0 2.0 2.0) _alpha)))))

(fn `UserConstructionScript`)